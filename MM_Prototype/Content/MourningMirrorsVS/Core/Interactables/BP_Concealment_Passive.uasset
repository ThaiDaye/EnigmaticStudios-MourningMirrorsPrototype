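; BP_Concealment_Passive is an interactable concealment volume that tracks whether the player is inside it.
; On BeginPlay it caches the first player character, cast to BP_Player, as its only valid occupant.
; Begin and end overlap events on the ActiveArea component set and clear the Occupied flag for that player.
; The Blueprint only maintains this flag and applies no concealment effect itself.
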(event `self.ReceiveBeginPlay`
  (bind _asbp_player (cast `/Game/MourningMirrorsVS/Core/Characters/BP_Player` (`GameplayStatics.GetPlayerCharacter` 0)))
  (set `self.ValidOccupants` _asbp_player))

(event `self.ActiveArea.OnComponentBeginOverlap`
  (params (OverlappedComponent :type "PrimitiveComponent Object Reference") (OtherActor :type "Actor Object Reference") (OtherComp :type "PrimitiveComponent Object Reference") (OtherBodyIndex :type Integer) (bFromSweep :type Boolean) (SweepResult :type "HitResult Structure (by ref)"))
  (if (== OtherActor (`self.ValidOccupants`))
    (set `self.bOccupied` true)))

(event `self.ActiveArea.OnComponentEndOverlap`
  (params (OverlappedComponent :type "PrimitiveComponent Object Reference") (OtherActor :type "Actor Object Reference") (OtherComp :type "PrimitiveComponent Object Reference") (OtherBodyIndex :type Integer))
  (if (== OtherActor (`self.ValidOccupants`))
    (set `self.bOccupied` false)))

(fn `UserConstructionScript`)