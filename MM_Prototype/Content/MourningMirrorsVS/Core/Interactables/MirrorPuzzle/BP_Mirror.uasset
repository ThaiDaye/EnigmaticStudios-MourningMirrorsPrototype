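; Puzzle mirror that emits an outgoing light beam matching the beam striking it.
; Each tick it checks overlaps and sets its ChildActor class, giving a plain BP_LightBeam priority over coloured beams.
; For coloured beams, the first overlap's BeamColour selects the matching beam subclass, with no class mapped for PURE.
; With no beam overlapping, it clears the child actor class.
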(event `self.ReceiveTick`
  (params (DeltaSeconds :type "Float (single-precision)"))
  (bind _overlappingactors (`self.GetOverlappingActors` "/Game/MourningMirrorsVS/Core/Interactables/MirrorPuzzle/ColourLightBeams/BP_LightBeam_Colour.BP_LightBeam_Colour_C"))
  (bind _childactor (`self.ChildActor`))
  (`parent.ReceiveTick` DeltaSeconds)
  (if (== (`KismetArrayLibrary.Array_Length` (`self.GetOverlappingActors` "/Game/MourningMirrorsVS/Core/Interactables/MirrorPuzzle/BP_LightBeam.BP_LightBeam_C")) 0)
    (if (== (`KismetArrayLibrary.Array_Length` _overlappingactors) 0)
      (`ChildActorComponent.SetChildActorClass` _childactor null :!label _label)
      (else
        (bind _asbp_light_beam_colour (cast `/Game/MourningMirrorsVS/Core/Interactables/MirrorPuzzle/ColourLightBeams/BP_LightBeam_Colour` (`|GetArrayItem` _overlappingactors))
          (:`then`
            (`ChildActorComponent.SetChildActorClass` _childactor (select `/Game/MourningMirrorsVS/Core/Interactables/MirrorPuzzle/ColourLightBeams/E_BeamColour` (`/Game/MourningMirrorsVS/Core/Interactables/MirrorPuzzle/ColourLightBeams/BP_LightBeam_Colour.Beam Colour` _asbp_light_beam_colour) :`NewEnumerator0` "/Game/MourningMirrorsVS/Core/Interactables/MirrorPuzzle/ColourLightBeams/BP_LightBeam_Red.BP_LightBeam_Red_C" :`NewEnumerator1` "/Game/MourningMirrorsVS/Core/Interactables/MirrorPuzzle/ColourLightBeams/BP_LightBeam_Yellow.BP_LightBeam_Yellow_C" :`NewEnumerator2` "/Game/MourningMirrorsVS/Core/Interactables/MirrorPuzzle/ColourLightBeams/BP_LightBeam_Blue.BP_LightBeam_Blue_C" :`NewEnumerator3` "/Game/MourningMirrorsVS/Core/Interactables/MirrorPuzzle/ColourLightBeams/BP_LightBeam_Orange.BP_LightBeam_Orange_C" :`NewEnumerator4` "/Game/MourningMirrorsVS/Core/Interactables/MirrorPuzzle/ColourLightBeams/BP_LightBeam_Purple.BP_LightBeam_Purple_C" :`NewEnumerator5` "/Game/MourningMirrorsVS/Core/Interactables/MirrorPuzzle/ColourLightBeams/BP_LightBeam_Green.BP_LightBeam_Green_C" :!type "Actor Class Reference")))
          (:`CastFailed`
            (goto _label)))))
    (else
      (`ChildActorComponent.SetChildActorClass` _childactor "/Game/MourningMirrorsVS/Core/Interactables/MirrorPuzzle/BP_LightBeam.BP_LightBeam_C"))))

(fn `UserConstructionScript`
  (`parent.UserConstructionScript`))