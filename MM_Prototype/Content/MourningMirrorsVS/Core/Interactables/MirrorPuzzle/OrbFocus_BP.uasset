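; Mirror puzzle focus orb that merges the light beams touching it and emits the resulting beam.
; Every Tick it polls overlapping beam actors, splitting each coloured beam into red, yellow and blue components.
; Those flags pick the ChildActor class: a primary, a mixed orange, purple or green, or a plain LightBeam when all three combine.
; An overlapping plain LightBeam overrides colour mixing, and no overlapping beams clears the output.
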(event `self.ReceiveTick`
  (params (DeltaSeconds :type "Float (single-precision)"))
  (bind _overlappingactors (`self.GetOverlappingActors` "/Game/MourningMirrorsVS/Core/Interactables/MirrorPuzzle/ColourLightBeams/ColourLightBeam_BP.ColourLightBeam_BP_C"))
  (bind _childactor (`self.ChildActor`))
  (bind _childactor_2 (`self.ChildActor`))
  (bind _hasred (`self.HasRed`))
  (bind _hasyellow (`self.HasYellow`))
  (bind _hasblue (`self.HasBlue`))
  (`parent.ReceiveTick` DeltaSeconds)
  (if (== (`KismetArrayLibrary.Array_Length` (`self.GetOverlappingActors` "/Game/MourningMirrorsVS/Core/Interactables/MirrorPuzzle/LightBeam_BP.LightBeam_BP_C")) 0)
    (if (== (`KismetArrayLibrary.Array_Length` _overlappingactors) 0)
      (`ChildActorComponent.SetChildActorClass` _childactor_2 null)
      (else
        (set `self.HasBlue` false)
        (set `self.HasYellow` false)
        (set `self.HasRed` false)
        (set `self.SourcesTouching` 0)
        (for _array_element _overlappingactors
          (bind _ascolour_light_beam_bp (cast `/Game/MourningMirrorsVS/Core/Interactables/MirrorPuzzle/ColourLightBeams/ColourLightBeam_BP` _array_element))
          (`|ExecutionSequence`
            (:`then_0`
              (bind _beam_colour (`/Game/MourningMirrorsVS/Core/Interactables/MirrorPuzzle/ColourLightBeams/ColourLightBeam_BP.Beam Colour` _ascolour_light_beam_bp))
              (if (or (`|EnumEquality` _beam_colour "NewEnumerator0") (`|EnumEquality` _beam_colour "NewEnumerator3") (`|EnumEquality` _beam_colour "NewEnumerator4"))
                (set `self.HasRed` true)
                (set `self.SourcesTouching` (+ (`self.SourcesTouching`) 1) :!label _label)))
            (:`then_1`
              (if (or (`|EnumEquality` _beam_colour "NewEnumerator1") (`|EnumEquality` _beam_colour "NewEnumerator3") (`|EnumEquality` _beam_colour "NewEnumerator5"))
                (set `self.HasYellow` true)
                (goto _label)))
            (:`then_2`
              (if (or (`|EnumEquality` _beam_colour "NewEnumerator2") (`|EnumEquality` _beam_colour "NewEnumerator4") (`|EnumEquality` _beam_colour "NewEnumerator5"))
                (set `self.HasBlue` true)
                (goto _label)))))
        ;[1 1 1] making light beam
        (if (and _hasred _hasyellow _hasblue)
          (`ChildActorComponent.SetChildActorClass` _childactor_2 "/Game/MourningMirrorsVS/Core/Interactables/MirrorPuzzle/LightBeam_BP.LightBeam_BP_C")
          (elif (== (`self.SourcesTouching`) 1)
            ;[1 1 1] MAKING PRIMARY COLOUR
            (if (`self.HasRed`)
              (`ChildActorComponent.SetChildActorClass` _childactor "/Game/MourningMirrorsVS/Core/Interactables/MirrorPuzzle/ColourLightBeams/RedLightBeam_BP.RedLightBeam_BP_C")
              ;[1 1 1] making orange
              (if (and _hasred _hasyellow) :!label _label_2
                (`ChildActorComponent.SetChildActorClass` _childactor "/Game/MourningMirrorsVS/Core/Interactables/MirrorPuzzle/ColourLightBeams/OrangeLightBeam_BP.OrangeLightBeam_BP_C")
                (else
                  ;[1 1 1] making PURPLE
                  (if (and _hasred _hasblue)
                    (`ChildActorComponent.SetChildActorClass` _childactor "/Game/MourningMirrorsVS/Core/Interactables/MirrorPuzzle/ColourLightBeams/PurpleLightBeam_BP.PurpleLightBeam_BP_C")
                    (else
                      ;[1 1 1] making GREEN
                      (if (and _hasyellow _hasblue)
                        (`ChildActorComponent.SetChildActorClass` _childactor "/Game/MourningMirrorsVS/Core/Interactables/MirrorPuzzle/ColourLightBeams/GreenLightBeam_BP.GreenLightBeam_BP_C"))))))
              (elif (`self.HasYellow`)
                (`ChildActorComponent.SetChildActorClass` _childactor "/Game/MourningMirrorsVS/Core/Interactables/MirrorPuzzle/ColourLightBeams/YellowLightBeam_BP.YellowLightBeam_BP_C")
                (goto _label_2)
                (elif (`self.HasBlue`)
                  (`ChildActorComponent.SetChildActorClass` _childactor "/Game/MourningMirrorsVS/Core/Interactables/MirrorPuzzle/ColourLightBeams/BlueLightBeam_BP.BlueLightBeam_BP_C")
                  (goto _label_2))))
            (else
              (goto _label_2))))))
    (else
      (`ChildActorComponent.SetChildActorClass` _childactor_2 "/Game/MourningMirrorsVS/Core/Interactables/MirrorPuzzle/LightBeam_BP.LightBeam_BP_C"))))

(fn `UserConstructionScript`
  (`parent.UserConstructionScript`))