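; BP_Prism is a mirror-puzzle prism that splits an incoming light beam into red, yellow and blue beams.
; Each Tick it polls overlapping beams and sets the classes of three child actor components to spawn or clear the outputs.
; A BP_LightBeam yields all three; otherwise the first BP_LightBeam_Colour's enum selects one of three primary pairs, without clearing the third output.
; No beam or any other colour clears all three.
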(event `self.ReceiveTick`
  (params (DeltaSeconds :type "Float (single-precision)"))
  (bind _overlappingactors (`self.GetOverlappingActors` "/Game/MourningMirrorsVS/Core/Interactables/MirrorPuzzle/ColourLightBeams/BP_LightBeam_Colour.BP_LightBeam_Colour_C"))
  (bind _red (`self.RED`))
  (bind _yellow (`self.YELLOW`))
  (bind _blue (`self.BLUE`))
  (bind _beam_colour (`/Game/MourningMirrorsVS/Core/Interactables/MirrorPuzzle/ColourLightBeams/BP_LightBeam_Colour.Beam Colour` (cast `/Game/MourningMirrorsVS/Core/Interactables/MirrorPuzzle/ColourLightBeams/BP_LightBeam_Colour` (`|GetArrayItem` _overlappingactors) :!pure true)))
  (`parent.ReceiveTick` DeltaSeconds)
  (if (== (`KismetArrayLibrary.Array_Length` (`self.GetOverlappingActors` "/Game/MourningMirrorsVS/Core/Interactables/MirrorPuzzle/BP_LightBeam.BP_LightBeam_C")) 0)
    (if (== (`KismetArrayLibrary.Array_Length` _overlappingactors) 0)
      (`ChildActorComponent.SetChildActorClass` _red null :!label _label)
      (`ChildActorComponent.SetChildActorClass` _yellow null)
      (`ChildActorComponent.SetChildActorClass` _blue null)
      (elif (`|EnumEquality` _beam_colour "NewEnumerator3")
        (`ChildActorComponent.SetChildActorClass` (`self.RED`) "/Game/MourningMirrorsVS/Core/Interactables/MirrorPuzzle/ColourLightBeams/BP_LightBeam_Red.BP_LightBeam_Red_C")
        (`ChildActorComponent.SetChildActorClass` (`self.YELLOW`) "/Game/MourningMirrorsVS/Core/Interactables/MirrorPuzzle/ColourLightBeams/BP_LightBeam_Yellow.BP_LightBeam_Yellow_C")
        (elif (`|EnumEquality` _beam_colour "NewEnumerator4")
          (`ChildActorComponent.SetChildActorClass` (`self.RED`) "/Game/MourningMirrorsVS/Core/Interactables/MirrorPuzzle/ColourLightBeams/BP_LightBeam_Red.BP_LightBeam_Red_C")
          (`ChildActorComponent.SetChildActorClass` (`self.BLUE`) "/Game/MourningMirrorsVS/Core/Interactables/MirrorPuzzle/ColourLightBeams/BP_LightBeam_Blue.BP_LightBeam_Blue_C")
          (elif (`|EnumEquality` _beam_colour "NewEnumerator5")
            (`ChildActorComponent.SetChildActorClass` (`self.YELLOW`) "/Game/MourningMirrorsVS/Core/Interactables/MirrorPuzzle/ColourLightBeams/BP_LightBeam_Yellow.BP_LightBeam_Yellow_C")
            (`ChildActorComponent.SetChildActorClass` (`self.BLUE`) "/Game/MourningMirrorsVS/Core/Interactables/MirrorPuzzle/ColourLightBeams/BP_LightBeam_Blue.BP_LightBeam_Blue_C")
            (else
              (goto _label))))))
    (else
      (`ChildActorComponent.SetChildActorClass` _red "/Game/MourningMirrorsVS/Core/Interactables/MirrorPuzzle/ColourLightBeams/BP_LightBeam_Red.BP_LightBeam_Red_C")
      (`ChildActorComponent.SetChildActorClass` _yellow "/Game/MourningMirrorsVS/Core/Interactables/MirrorPuzzle/ColourLightBeams/BP_LightBeam_Yellow.BP_LightBeam_Yellow_C")
      (`ChildActorComponent.SetChildActorClass` _blue "/Game/MourningMirrorsVS/Core/Interactables/MirrorPuzzle/ColourLightBeams/BP_LightBeam_Blue.BP_LightBeam_Blue_C"))))

(fn `UserConstructionScript`
  (`parent.UserConstructionScript`))