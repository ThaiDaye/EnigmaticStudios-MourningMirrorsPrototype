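; BP_LightBeam is a light beam actor for the mirror puzzle that visually stretches to the first surface it hits.
; Each Tick it runs a forward sphere trace on the Visibility channel from the actor location.
; On a blocking hit, it centers the Cylinder between origin and impact point and scales its Z to that distance.
; It then casts the hit actor to BP_Mirror, but nothing follows the cast.
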(event `self.ReceiveTick`
  (params (DeltaSeconds :type "Float (single-precision)"))
  (bind _returnvalue (`self.K2_GetActorLocation`))
  (bind _cylinder (`self.Cylinder`))
  (bind _outhit (`KismetSystemLibrary.SphereTraceSingle` :`Start` _returnvalue :`End` (+ _returnvalue (* (`SceneComponent.GetForwardVector` (`self.DefaultSceneRoot`)) 10000.0)) :`Radius` 30.0 :`TraceChannel` "TraceTypeQuery1" :`bTraceComplex` true :`TraceColor` (struct :`R` 1.0 :`G` 0.34375 :`B` 0.34375 :`A` 1.0) :`TraceHitColor` (struct :`R` 1.0 :`G` 0.739724 :`B` 0.071455 :`A` 1.0)))
  (bind (_bblockinghit _binitialoverlap _time _distance _location _impactpoint _normal _impactnormal _physmat _hitactor) (`GameplayStatics.BreakHitResult` _outhit))
  (if _bblockinghit
    (`SceneComponent.K2_SetWorldLocation` _cylinder (+ (/ _returnvalue 2.0) (/ _impactpoint 2.0)) false false)
    (`SceneComponent.SetWorldScale3D` _cylinder (`KismetMathLibrary.MakeVector` (.x (`SceneComponent.K2_GetComponentScale` (`self.Cylinder`))) (.y (`SceneComponent.K2_GetComponentScale` (`self.Cylinder`))) (* (`KismetMathLibrary.VSize` (- _returnvalue _impactpoint)) 0.01)))
    (cast `/Game/MourningMirrorsVS/Core/Interactables/MirrorPuzzle/BP_Mirror` _hitactor)))

(fn `UserConstructionScript`)