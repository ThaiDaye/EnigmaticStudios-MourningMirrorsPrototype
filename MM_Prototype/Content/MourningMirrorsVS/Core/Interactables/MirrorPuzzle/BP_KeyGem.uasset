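; BP_KeyGem is a mirror-puzzle gem that activates when struck by a light beam matching its KeyColour.
; Each Tick polls beam overlaps, with plain beams taking priority and matching only PURE, then swaps the Cube material between mirror and coloured glow.
; On a match, a child actor becomes a same-coloured beam, kept only if SpawnBeaconOnActive is set.
; Without a match the child is cleared, and activation persists unless NeedsConstantLight is set.
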(event `self.ReceiveBeginPlay`
  ;[1 1 1] set key colour
  (`PrimitiveComponent.SetSimulatePhysics` (`self.Cube`) false)
  (`PrimitiveComponent.SetMaterial` (`self.StaticMesh`) 1 (select `/Game/MourningMirrorsVS/Core/Interactables/MirrorPuzzle/ColourLightBeams/E_BeamColour` (`self.KeyColour`) :`NewEnumerator0` "/Game/MourningMirrorsVS/MaterialLibrary/LightBeam/MI_LightGlow_Red.MI_LightGlow_Red" :`NewEnumerator1` "/Game/MourningMirrorsVS/MaterialLibrary/LightBeam/MI_LightGlow_Yellow.MI_LightGlow_Yellow" :`NewEnumerator2` "/Game/MourningMirrorsVS/MaterialLibrary/LightBeam/MI_LightGlow_Blue.MI_LightGlow_Blue" :`NewEnumerator3` "/Game/MourningMirrorsVS/MaterialLibrary/LightBeam/MI_LightGlow_Orange.MI_LightGlow_Orange" :`NewEnumerator4` "/Game/MourningMirrorsVS/MaterialLibrary/LightBeam/MI_LightGlow_Purple.MI_LightGlow_Purple" :`NewEnumerator5` "/Game/MourningMirrorsVS/MaterialLibrary/LightBeam/MI_LightGlow_Green.MI_LightGlow_Green" :`NewEnumerator6` "/Game/MourningMirrorsVS/MaterialLibrary/LightBeam/MI_LightGlow_02.MI_LightGlow_02" :!type "MaterialInterface Object Reference")))

(event `self.ReceiveTick`
  (params (DeltaSeconds :type "Float (single-precision)"))
  (bind _overlappingactors (`self.GetOverlappingActors` "/Game/MourningMirrorsVS/Core/Interactables/MirrorPuzzle/ColourLightBeams/BP_LightBeam_Colour.BP_LightBeam_Colour_C"))
  (bind _childactor (`self.ChildActor`))
  (bind _cube (`self.Cube`))
  (`parent.ReceiveTick` DeltaSeconds)
  (if (`self.Activated`)
    (`PrimitiveComponent.SetMaterial` _cube 0 (select `/Game/MourningMirrorsVS/Core/Interactables/MirrorPuzzle/ColourLightBeams/E_BeamColour` (`self.KeyColour`) :`NewEnumerator0` "/Game/MourningMirrorsVS/MaterialLibrary/LightBeam/MI_LightGlow_Red.MI_LightGlow_Red" :`NewEnumerator1` "/Game/MourningMirrorsVS/MaterialLibrary/LightBeam/MI_LightGlow_Yellow.MI_LightGlow_Yellow" :`NewEnumerator2` "/Game/MourningMirrorsVS/MaterialLibrary/LightBeam/MI_LightGlow_Blue.MI_LightGlow_Blue" :`NewEnumerator3` "/Game/MourningMirrorsVS/MaterialLibrary/LightBeam/MI_LightGlow_Orange.MI_LightGlow_Orange" :`NewEnumerator4` "/Game/MourningMirrorsVS/MaterialLibrary/LightBeam/MI_LightGlow_Purple.MI_LightGlow_Purple" :`NewEnumerator5` "/Game/MourningMirrorsVS/MaterialLibrary/LightBeam/MI_LightGlow_Green.MI_LightGlow_Green" :`NewEnumerator6` "/Game/MourningMirrorsVS/MaterialLibrary/LightBeam/MI_LightGlow_02.MI_LightGlow_02" :!type "MaterialInterface Object Reference"))
    (else
      (`PrimitiveComponent.SetMaterial` _cube 0 "/Game/MourningMirrorsVS/MaterialLibrary/MI_Mirror_Full.MI_Mirror_Full")))
  (if (== (`KismetArrayLibrary.Array_Length` (`self.GetOverlappingActors` "/Game/MourningMirrorsVS/Core/Interactables/MirrorPuzzle/BP_LightBeam.BP_LightBeam_C")) 0)
    (if (== (`KismetArrayLibrary.Array_Length` _overlappingactors) 0)
      (`ChildActorComponent.SetChildActorClass` _childactor null :!label _label)
      (if (`self.NeedsConstantLight`)
        (set `self.Activated` false))
      (else
        (bind _asbp_light_beam_colour (cast `/Game/MourningMirrorsVS/Core/Interactables/MirrorPuzzle/ColourLightBeams/BP_LightBeam_Colour` (`|GetArrayItem` _overlappingactors))
          (:`then`
            (bind _beam_colour (`/Game/MourningMirrorsVS/Core/Interactables/MirrorPuzzle/ColourLightBeams/BP_LightBeam_Colour.Beam Colour` _asbp_light_beam_colour))
            (if (`|EnumEquality` (`self.KeyColour`) _beam_colour)
              (`ChildActorComponent.SetChildActorClass` _childactor (select `/Game/MourningMirrorsVS/Core/Interactables/MirrorPuzzle/ColourLightBeams/E_BeamColour` _beam_colour :`NewEnumerator0` "/Game/MourningMirrorsVS/Core/Interactables/MirrorPuzzle/ColourLightBeams/BP_LightBeam_Red.BP_LightBeam_Red_C" :`NewEnumerator1` "/Game/MourningMirrorsVS/Core/Interactables/MirrorPuzzle/ColourLightBeams/BP_LightBeam_Yellow.BP_LightBeam_Yellow_C" :`NewEnumerator2` "/Game/MourningMirrorsVS/Core/Interactables/MirrorPuzzle/ColourLightBeams/BP_LightBeam_Blue.BP_LightBeam_Blue_C" :`NewEnumerator3` "/Game/MourningMirrorsVS/Core/Interactables/MirrorPuzzle/ColourLightBeams/BP_LightBeam_Orange.BP_LightBeam_Orange_C" :`NewEnumerator4` "/Game/MourningMirrorsVS/Core/Interactables/MirrorPuzzle/ColourLightBeams/BP_LightBeam_Purple.BP_LightBeam_Purple_C" :`NewEnumerator5` "/Game/MourningMirrorsVS/Core/Interactables/MirrorPuzzle/ColourLightBeams/BP_LightBeam_Green.BP_LightBeam_Green_C" :!type "Actor Class Reference"))
              (set `self.Activated` true)
              (if (not (`self.SpawnBeaconOnActive`)) :!label _label_2
                (`ChildActorComponent.SetChildActorClass` _childactor null))
              (else
                (goto _label))))
          (:`CastFailed`
            (goto _label)))))
    (elif (`|EnumEquality` (`self.KeyColour`) "NewEnumerator6")
      (`ChildActorComponent.SetChildActorClass` _childactor "/Game/MourningMirrorsVS/Core/Interactables/MirrorPuzzle/BP_LightBeam.BP_LightBeam_C")
      (set `self.Activated` true)
      (goto _label_2)
      (else
        (goto _label)))))

(fn `UserConstructionScript`
  (`parent.UserConstructionScript`))