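; BP_OrbFocus is a mirror puzzle orb that merges the light beams touching it into one output beam.
; Every Tick it checks overlapping beams, breaking coloured ones into red, yellow and blue flags.
; It then sets its ChildActor class to the mixed result: a primary, orange, purple, green, or plain BP_LightBeam for all three.
; An overlapping plain beam overrides the mix, and no beams clears the output.
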(event `self.ReceiveTick`
  (params (DeltaSeconds :type "Float (single-precision)"))
  (bind _overlappingactors (`self.GetOverlappingActors` "/Game/MourningMirrorsVS/Core/Interactables/MirrorPuzzle/ColourLightBeams/BP_LightBeam_Colour.BP_LightBeam_Colour_C"))
  (bind _childactor (`self.ChildActor`))
  (bind _childactor_2 (`self.ChildActor`))
  (bind _hasred (`self.HasRed`))
  (bind _hasyellow (`self.HasYellow`))
  (bind _hasblue (`self.HasBlue`))
  (`parent.ReceiveTick` DeltaSeconds)
  (if (== (`KismetArrayLibrary.Array_Length` (`self.GetOverlappingActors` "/Game/MourningMirrorsVS/Core/Interactables/MirrorPuzzle/BP_LightBeam.BP_LightBeam_C")) 0)
    (if (== (`KismetArrayLibrary.Array_Length` _overlappingactors) 0)
      (`ChildActorComponent.SetChildActorClass` _childactor_2 null)
      (else
        (set `self.HasBlue` false)
        (set `self.HasYellow` false)
        (set `self.HasRed` false)
        (set `self.SourcesTouching` 0)
        (for _array_element _overlappingactors
          (bind _asbp_light_beam_colour (cast `/Game/MourningMirrorsVS/Core/Interactables/MirrorPuzzle/ColourLightBeams/BP_LightBeam_Colour` _array_element))
          (`|ExecutionSequence`
            (:`then_0`
              (bind _beam_colour (`/Game/MourningMirrorsVS/Core/Interactables/MirrorPuzzle/ColourLightBeams/BP_LightBeam_Colour.Beam Colour` _asbp_light_beam_colour))
              (if (or (`|EnumEquality` _beam_colour "NewEnumerator0") (`|EnumEquality` _beam_colour "NewEnumerator3") (`|EnumEquality` _beam_colour "NewEnumerator4"))
                (set `self.HasRed` true)
                (set `self.SourcesTouching` (+ (`self.SourcesTouching`) 1) :!label _label)))
            (:`then_1`
              (if (or (`|EnumEquality` _beam_colour "NewEnumerator1") (`|EnumEquality` _beam_colour "NewEnumerator3") (`|EnumEquality` _beam_colour "NewEnumerator5"))
                (set `self.HasYellow` true)
                (goto _label)))
            (:`then_2`
              (if (or (`|EnumEquality` _beam_colour "NewEnumerator2") (`|EnumEquality` _beam_colour "NewEnumerator4") (`|EnumEquality` _beam_colour "NewEnumerator5"))
                (set `self.HasBlue` true)
                (goto _label)))))
        ;[1 1 1] making light beam
        (if (and _hasred _hasyellow _hasblue)
          (`ChildActorComponent.SetChildActorClass` _childactor_2 "/Game/MourningMirrorsVS/Core/Interactables/MirrorPuzzle/BP_LightBeam.BP_LightBeam_C")
          (elif (== (`self.SourcesTouching`) 1)
            ;[1 1 1] MAKING PRIMARY COLOUR
            (if (`self.HasRed`)
              (`ChildActorComponent.SetChildActorClass` _childactor "/Game/MourningMirrorsVS/Core/Interactables/MirrorPuzzle/ColourLightBeams/BP_LightBeam_Red.BP_LightBeam_Red_C")
              ;[1 1 1] making orange
              (if (and _hasred _hasyellow) :!label _label_2
                (`ChildActorComponent.SetChildActorClass` _childactor "/Game/MourningMirrorsVS/Core/Interactables/MirrorPuzzle/ColourLightBeams/BP_LightBeam_Orange.BP_LightBeam_Orange_C")
                (else
                  ;[1 1 1] making PURPLE
                  (if (and _hasred _hasblue)
                    (`ChildActorComponent.SetChildActorClass` _childactor "/Game/MourningMirrorsVS/Core/Interactables/MirrorPuzzle/ColourLightBeams/BP_LightBeam_Purple.BP_LightBeam_Purple_C")
                    (else
                      ;[1 1 1] making GREEN
                      (if (and _hasyellow _hasblue)
                        (`ChildActorComponent.SetChildActorClass` _childactor "/Game/MourningMirrorsVS/Core/Interactables/MirrorPuzzle/ColourLightBeams/BP_LightBeam_Green.BP_LightBeam_Green_C"))))))
              (elif (`self.HasYellow`)
                (`ChildActorComponent.SetChildActorClass` _childactor "/Game/MourningMirrorsVS/Core/Interactables/MirrorPuzzle/ColourLightBeams/BP_LightBeam_Yellow.BP_LightBeam_Yellow_C")
                (goto _label_2)
                (elif (`self.HasBlue`)
                  (`ChildActorComponent.SetChildActorClass` _childactor "/Game/MourningMirrorsVS/Core/Interactables/MirrorPuzzle/ColourLightBeams/BP_LightBeam_Blue.BP_LightBeam_Blue_C")
                  (goto _label_2))))
            (else
              (goto _label_2))))))
    (else
      (`ChildActorComponent.SetChildActorClass` _childactor_2 "/Game/MourningMirrorsVS/Core/Interactables/MirrorPuzzle/BP_LightBeam.BP_LightBeam_C"))))

(fn `UserConstructionScript`
  (`parent.UserConstructionScript`))