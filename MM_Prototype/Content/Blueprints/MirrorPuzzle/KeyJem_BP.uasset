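; KeyJem_BP is a colour-keyed gem for the mirror puzzle that activates when hit by a light beam of its KeyColour.
; Each tick it checks overlapping beams, with plain LightBeam_BP matching only PURE keys and taking priority over coloured beams.
; A match lights the cube and, if SpawnBeaconOnActive, emits a same-coloured beam through a child actor.
; Without a match that beam clears, and activation persists unless NeedsConstantLight is set.
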(event `self.ReceiveBeginPlay`
  ;[1 1 1] set key colour
  (`PrimitiveComponent.SetSimulatePhysics` (`self.Cube`) false)
  (`PrimitiveComponent.SetMaterial` (`self.StaticMesh`) 1 (select `/Game/Blueprints/MirrorPuzzle/ColourLightBeams/BeamColour_Enum` (`self.KeyColour`) :`NewEnumerator0` "/Game/Materials/LightBeamMaterial/LightGlow_Mat_Red.LightGlow_Mat_Red" :`NewEnumerator1` "/Game/Materials/LightBeamMaterial/LightGlow_Mat_Yellow.LightGlow_Mat_Yellow" :`NewEnumerator2` "/Game/Materials/LightBeamMaterial/LightGlow_Mat_BLue.LightGlow_Mat_BLue" :`NewEnumerator3` "/Game/Materials/LightBeamMaterial/LightGlow_Mat_Orange.LightGlow_Mat_Orange" :`NewEnumerator4` "/Game/Materials/LightBeamMaterial/LightGlow_Mat_Purple.LightGlow_Mat_Purple" :`NewEnumerator5` "/Game/Materials/LightBeamMaterial/LightGlow_Mat_Green.LightGlow_Mat_Green" :`NewEnumerator6` "/Game/Materials/LightBeamMaterial/LightGlow_Mat_Inst1.LightGlow_Mat_Inst1" :!type "MaterialInterface Object Reference")))

(event `self.ReceiveTick`
  (params (DeltaSeconds :type "Float (single-precision)"))
  (bind _overlappingactors (`self.GetOverlappingActors` "/Game/Blueprints/MirrorPuzzle/ColourLightBeams/ColourLightBeam_BP.ColourLightBeam_BP_C"))
  (bind _childactor (`self.ChildActor`))
  (bind _cube (`self.Cube`))
  (`parent.ReceiveTick` DeltaSeconds)
  (if (`self.Activated`)
    (`PrimitiveComponent.SetMaterial` _cube 0 (select `/Game/Blueprints/MirrorPuzzle/ColourLightBeams/BeamColour_Enum` (`self.KeyColour`) :`NewEnumerator0` "/Game/Materials/LightBeamMaterial/LightGlow_Mat_Red.LightGlow_Mat_Red" :`NewEnumerator1` "/Game/Materials/LightBeamMaterial/LightGlow_Mat_Yellow.LightGlow_Mat_Yellow" :`NewEnumerator2` "/Game/Materials/LightBeamMaterial/LightGlow_Mat_BLue.LightGlow_Mat_BLue" :`NewEnumerator3` "/Game/Materials/LightBeamMaterial/LightGlow_Mat_Orange.LightGlow_Mat_Orange" :`NewEnumerator4` "/Game/Materials/LightBeamMaterial/LightGlow_Mat_Purple.LightGlow_Mat_Purple" :`NewEnumerator5` "/Game/Materials/LightBeamMaterial/LightGlow_Mat_Green.LightGlow_Mat_Green" :`NewEnumerator6` "/Game/Materials/LightBeamMaterial/LightGlow_Mat_Inst1.LightGlow_Mat_Inst1" :!type "MaterialInterface Object Reference"))
    (else
      (`PrimitiveComponent.SetMaterial` _cube 0 "/Game/Materials/Mirror.Mirror")))
  (if (== (`KismetArrayLibrary.Array_Length` (`self.GetOverlappingActors` "/Game/Blueprints/MirrorPuzzle/LightBeam_BP.LightBeam_BP_C")) 0)
    (if (== (`KismetArrayLibrary.Array_Length` _overlappingactors) 0)
      (`ChildActorComponent.SetChildActorClass` _childactor null :!label _label)
      (if (`self.NeedsConstantLight`)
        (set `self.Activated` false))
      (else
        (bind _ascolour_light_beam_bp (cast `/Game/Blueprints/MirrorPuzzle/ColourLightBeams/ColourLightBeam_BP` (`|GetArrayItem` _overlappingactors))
          (:`then`
            (bind _beam_colour (`/Game/Blueprints/MirrorPuzzle/ColourLightBeams/ColourLightBeam_BP.Beam Colour` _ascolour_light_beam_bp))
            (if (`|EnumEquality` (`self.KeyColour`) _beam_colour)
              (`ChildActorComponent.SetChildActorClass` _childactor (select `/Game/Blueprints/MirrorPuzzle/ColourLightBeams/BeamColour_Enum` _beam_colour :`NewEnumerator0` "/Game/Blueprints/MirrorPuzzle/ColourLightBeams/RedLightBeam_BP.RedLightBeam_BP_C" :`NewEnumerator1` "/Game/Blueprints/MirrorPuzzle/ColourLightBeams/YellowLightBeam_BP.YellowLightBeam_BP_C" :`NewEnumerator2` "/Game/Blueprints/MirrorPuzzle/ColourLightBeams/BlueLightBeam_BP.BlueLightBeam_BP_C" :`NewEnumerator3` "/Game/Blueprints/MirrorPuzzle/ColourLightBeams/OrangeLightBeam_BP.OrangeLightBeam_BP_C" :`NewEnumerator4` "/Game/Blueprints/MirrorPuzzle/ColourLightBeams/PurpleLightBeam_BP.PurpleLightBeam_BP_C" :`NewEnumerator5` "/Game/Blueprints/MirrorPuzzle/ColourLightBeams/GreenLightBeam_BP.GreenLightBeam_BP_C" :!type "Actor Class Reference"))
              (set `self.Activated` true)
              (if (not (`self.SpawnBeaconOnActive`)) :!label _label_2
                (`ChildActorComponent.SetChildActorClass` _childactor null))
              (else
                (goto _label))))
          (:`CastFailed`
            (goto _label)))))
    (elif (`|EnumEquality` (`self.KeyColour`) "NewEnumerator6")
      (`ChildActorComponent.SetChildActorClass` _childactor "/Game/Blueprints/MirrorPuzzle/LightBeam_BP.LightBeam_BP_C")
      (set `self.Activated` true)
      (goto _label_2)
      (else
        (goto _label)))))

(fn `UserConstructionScript`
  (`parent.UserConstructionScript`))