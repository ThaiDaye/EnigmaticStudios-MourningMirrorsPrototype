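; Mirror puzzle actor that re-emits an incoming light beam through a child actor component.
; Every tick it checks its overlaps and sets the child actor class to the plain light beam if one overlaps.
; Otherwise it matches the first overlapping coloured beam's colour to a beam subclass, with no class mapped for Pure.
; With no beam overlapping, the child actor class is cleared.
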(event `self.ReceiveTick`
  (params (DeltaSeconds :type "Float (single-precision)"))
  (bind _overlappingactors (`self.GetOverlappingActors` "/Game/Blueprints/MirrorPuzzle/ColourLightBeams/ColourLightBeam_BP.ColourLightBeam_BP_C"))
  (bind _childactor (`self.ChildActor`))
  (`parent.ReceiveTick` DeltaSeconds)
  (if (== (`KismetArrayLibrary.Array_Length` (`self.GetOverlappingActors` "/Game/Blueprints/MirrorPuzzle/LightBeam_BP.LightBeam_BP_C")) 0)
    (if (== (`KismetArrayLibrary.Array_Length` _overlappingactors) 0)
      (`ChildActorComponent.SetChildActorClass` _childactor null :!label _label)
      (else
        (bind _ascolour_light_beam_bp (cast `/Game/Blueprints/MirrorPuzzle/ColourLightBeams/ColourLightBeam_BP` (`|GetArrayItem` _overlappingactors))
          (:`then`
            (`ChildActorComponent.SetChildActorClass` _childactor (select `/Game/Blueprints/MirrorPuzzle/ColourLightBeams/BeamColour_Enum` (`/Game/Blueprints/MirrorPuzzle/ColourLightBeams/ColourLightBeam_BP.Beam Colour` _ascolour_light_beam_bp) :`NewEnumerator0` "/Game/Blueprints/MirrorPuzzle/ColourLightBeams/RedLightBeam_BP.RedLightBeam_BP_C" :`NewEnumerator1` "/Game/Blueprints/MirrorPuzzle/ColourLightBeams/YellowLightBeam_BP.YellowLightBeam_BP_C" :`NewEnumerator2` "/Game/Blueprints/MirrorPuzzle/ColourLightBeams/BlueLightBeam_BP.BlueLightBeam_BP_C" :`NewEnumerator3` "/Game/Blueprints/MirrorPuzzle/ColourLightBeams/OrangeLightBeam_BP.OrangeLightBeam_BP_C" :`NewEnumerator4` "/Game/Blueprints/MirrorPuzzle/ColourLightBeams/PurpleLightBeam_BP.PurpleLightBeam_BP_C" :`NewEnumerator5` "/Game/Blueprints/MirrorPuzzle/ColourLightBeams/GreenLightBeam_BP.GreenLightBeam_BP_C" :!type "Actor Class Reference")))
          (:`CastFailed`
            (goto _label)))))
    (else
      (`ChildActorComponent.SetChildActorClass` _childactor "/Game/Blueprints/MirrorPuzzle/LightBeam_BP.LightBeam_BP_C"))))

(fn `UserConstructionScript`
  (`parent.UserConstructionScript`))