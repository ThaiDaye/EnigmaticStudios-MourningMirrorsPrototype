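; Coloured mirror for a light-beam puzzle that emits a beam filtered by its MirrorColour, which also picks its glow material on BeginPlay.
; Each Tick it checks overlapping beams and swaps its ChildActor class to the outgoing beam, or clears it.
; An overlapping LightBeam_BP takes priority and yields the mirror's colour.
; Otherwise the first coloured beam passes if it matches, and orange, purple or green beams yield their red, yellow or blue component.
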(event `self.ReceiveBeginPlay`
  ;[1 1 1] set mirror colour
  (`PrimitiveComponent.SetMaterial` (`self.Cube`) 1 (select `/Game/Blueprints/MirrorPuzzle/ColourLightBeams/BeamColour_Enum` (`self.MirrorColour`) :`NewEnumerator0` "/Game/Materials/LightBeamMaterial/LightGlow_Mat_Red.LightGlow_Mat_Red" :`NewEnumerator1` "/Game/Materials/LightBeamMaterial/LightGlow_Mat_Yellow.LightGlow_Mat_Yellow" :`NewEnumerator2` "/Game/Materials/LightBeamMaterial/LightGlow_Mat_BLue.LightGlow_Mat_BLue" :`NewEnumerator3` "/Game/Materials/LightBeamMaterial/LightGlow_Mat_Orange.LightGlow_Mat_Orange" :`NewEnumerator4` "/Game/Materials/LightBeamMaterial/LightGlow_Mat_Purple.LightGlow_Mat_Purple" :`NewEnumerator5` "/Game/Materials/LightBeamMaterial/LightGlow_Mat_Green.LightGlow_Mat_Green" :!type "MaterialInterface Object Reference")))

(event `self.ReceiveTick`
  (params (DeltaSeconds :type "Float (single-precision)"))
  (bind _overlappingactors (`self.GetOverlappingActors` "/Game/Blueprints/MirrorPuzzle/ColourLightBeams/ColourLightBeam_BP.ColourLightBeam_BP_C"))
  (bind _childactor (`self.ChildActor`))
  (bind _childactor_2 (`self.ChildActor`))
  (bind _mirrorcolour (`self.MirrorColour`))
  (bind _childactor_3 (`self.ChildActor`))
  (`parent.ReceiveTick` DeltaSeconds)
  (if (== (`KismetArrayLibrary.Array_Length` (`self.GetOverlappingActors` "/Game/Blueprints/MirrorPuzzle/LightBeam_BP.LightBeam_BP_C")) 0)
    (if (== (`KismetArrayLibrary.Array_Length` _overlappingactors) 0)
      (`ChildActorComponent.SetChildActorClass` (`self.ChildActor`) null :!label _label)
      (else
        (bind _ascolour_light_beam_bp (cast `/Game/Blueprints/MirrorPuzzle/ColourLightBeams/ColourLightBeam_BP` (`|GetArrayItem` _overlappingactors))
          (:`then`
            (bind _beam_colour (`/Game/Blueprints/MirrorPuzzle/ColourLightBeams/ColourLightBeam_BP.Beam Colour` _ascolour_light_beam_bp))
            (if (`|EnumEquality` _beam_colour _mirrorcolour)
              (`ChildActorComponent.SetChildActorClass` (`self.ChildActor`) (select `/Game/Blueprints/MirrorPuzzle/ColourLightBeams/BeamColour_Enum` _beam_colour :`NewEnumerator0` "/Game/Blueprints/MirrorPuzzle/ColourLightBeams/RedLightBeam_BP.RedLightBeam_BP_C" :`NewEnumerator1` "/Game/Blueprints/MirrorPuzzle/ColourLightBeams/YellowLightBeam_BP.YellowLightBeam_BP_C" :`NewEnumerator2` "/Game/Blueprints/MirrorPuzzle/ColourLightBeams/BlueLightBeam_BP.BlueLightBeam_BP_C" :`NewEnumerator3` "/Game/Blueprints/MirrorPuzzle/ColourLightBeams/OrangeLightBeam_BP.OrangeLightBeam_BP_C" :`NewEnumerator4` "/Game/Blueprints/MirrorPuzzle/ColourLightBeams/PurpleLightBeam_BP.PurpleLightBeam_BP_C" :`NewEnumerator5` "/Game/Blueprints/MirrorPuzzle/ColourLightBeams/GreenLightBeam_BP.GreenLightBeam_BP_C" :!type "Actor Class Reference"))
              (elif (or (`|EnumEquality` _beam_colour "NewEnumerator3") (`|EnumEquality` _beam_colour "NewEnumerator4") (`|EnumEquality` _beam_colour "NewEnumerator5"))
                (switch `/Game/Blueprints/MirrorPuzzle/ColourLightBeams/BeamColour_Enum` _mirrorcolour
                  (:`NewEnumerator0`
                    ;[1 1 1] reflect only Red light
                    (if (or (`|EnumEquality` _beam_colour "NewEnumerator3") (`|EnumEquality` _beam_colour "NewEnumerator4"))
                      (`ChildActorComponent.SetChildActorClass` _childactor_3 "/Game/Blueprints/MirrorPuzzle/ColourLightBeams/RedLightBeam_BP.RedLightBeam_BP_C")
                      (else
                        (`ChildActorComponent.SetChildActorClass` _childactor_3 null))))
                  (:`NewEnumerator1`
                    ;[1 1 1] reflect only yellow light
                    (if (or (`|EnumEquality` _beam_colour "NewEnumerator3") (`|EnumEquality` _beam_colour "NewEnumerator5"))
                      (`ChildActorComponent.SetChildActorClass` _childactor_2 "/Game/Blueprints/MirrorPuzzle/ColourLightBeams/YellowLightBeam_BP.YellowLightBeam_BP_C")
                      (else
                        (`ChildActorComponent.SetChildActorClass` _childactor_2 null))))
                  (:`NewEnumerator2`
                    ;[1 1 1] reflect only blue light
                    (if (or (`|EnumEquality` _beam_colour "NewEnumerator4") (`|EnumEquality` _beam_colour "NewEnumerator5"))
                      (`ChildActorComponent.SetChildActorClass` _childactor "/Game/Blueprints/MirrorPuzzle/ColourLightBeams/BlueLightBeam_BP.BlueLightBeam_BP_C")
                      (else
                        (`ChildActorComponent.SetChildActorClass` _childactor null)))))
                (else
                  (goto _label)))))
          (:`CastFailed`
            (goto _label)))))
    (else
      ;[1 1 1] refleact light beam
      (`ChildActorComponent.SetChildActorClass` (`self.ChildActor`) (select `/Game/Blueprints/MirrorPuzzle/ColourLightBeams/BeamColour_Enum` (`self.MirrorColour`) :`NewEnumerator0` "/Game/Blueprints/MirrorPuzzle/ColourLightBeams/RedLightBeam_BP.RedLightBeam_BP_C" :`NewEnumerator1` "/Game/Blueprints/MirrorPuzzle/ColourLightBeams/YellowLightBeam_BP.YellowLightBeam_BP_C" :`NewEnumerator2` "/Game/Blueprints/MirrorPuzzle/ColourLightBeams/BlueLightBeam_BP.BlueLightBeam_BP_C" :`NewEnumerator3` "/Game/Blueprints/MirrorPuzzle/ColourLightBeams/OrangeLightBeam_BP.OrangeLightBeam_BP_C" :`NewEnumerator4` "/Game/Blueprints/MirrorPuzzle/ColourLightBeams/PurpleLightBeam_BP.PurpleLightBeam_BP_C" :`NewEnumerator5` "/Game/Blueprints/MirrorPuzzle/ColourLightBeams/GreenLightBeam_BP.GreenLightBeam_BP_C" :!type "Actor Class Reference")))))

(fn `UserConstructionScript`
  (`parent.UserConstructionScript`))