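; Prism puzzle piece that splits incoming light beams into red, yellow and blue beams through three child actor components.
; Each Tick polls overlaps: a LightBeam_BP spawns all three colours, taking priority over any ColourLightBeam_BP.
; Otherwise, the first coloured beam's BeamColour selects one of three colour pairs, without clearing the third component.
; No beam or any other colour clears all three child actor classes.
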(event `self.ReceiveTick`
  (params (DeltaSeconds :type "Float (single-precision)"))
  (bind _overlappingactors (`self.GetOverlappingActors` "/Game/Blueprints/MirrorPuzzle/ColourLightBeams/ColourLightBeam_BP.ColourLightBeam_BP_C"))
  (bind _red (`self.RED`))
  (bind _yellow (`self.YELLOW`))
  (bind _blue (`self.BLUE`))
  (bind _beam_colour (`/Game/Blueprints/MirrorPuzzle/ColourLightBeams/ColourLightBeam_BP.Beam Colour` (cast `/Game/Blueprints/MirrorPuzzle/ColourLightBeams/ColourLightBeam_BP` (`|GetArrayItem` _overlappingactors) :!pure true)))
  (`parent.ReceiveTick` DeltaSeconds)
  (if (== (`KismetArrayLibrary.Array_Length` (`self.GetOverlappingActors` "/Game/Blueprints/MirrorPuzzle/LightBeam_BP.LightBeam_BP_C")) 0)
    (if (== (`KismetArrayLibrary.Array_Length` _overlappingactors) 0)
      (`ChildActorComponent.SetChildActorClass` _red null :!label _label)
      (`ChildActorComponent.SetChildActorClass` _yellow null)
      (`ChildActorComponent.SetChildActorClass` _blue null)
      (elif (`|EnumEquality` _beam_colour "NewEnumerator3")
        (`ChildActorComponent.SetChildActorClass` (`self.RED`) "/Game/Blueprints/MirrorPuzzle/ColourLightBeams/RedLightBeam_BP.RedLightBeam_BP_C")
        (`ChildActorComponent.SetChildActorClass` (`self.YELLOW`) "/Game/Blueprints/MirrorPuzzle/ColourLightBeams/YellowLightBeam_BP.YellowLightBeam_BP_C")
        (elif (`|EnumEquality` _beam_colour "NewEnumerator4")
          (`ChildActorComponent.SetChildActorClass` (`self.RED`) "/Game/Blueprints/MirrorPuzzle/ColourLightBeams/RedLightBeam_BP.RedLightBeam_BP_C")
          (`ChildActorComponent.SetChildActorClass` (`self.BLUE`) "/Game/Blueprints/MirrorPuzzle/ColourLightBeams/BlueLightBeam_BP.BlueLightBeam_BP_C")
          (elif (`|EnumEquality` _beam_colour "NewEnumerator5")
            (`ChildActorComponent.SetChildActorClass` (`self.YELLOW`) "/Game/Blueprints/MirrorPuzzle/ColourLightBeams/YellowLightBeam_BP.YellowLightBeam_BP_C")
            (`ChildActorComponent.SetChildActorClass` (`self.BLUE`) "/Game/Blueprints/MirrorPuzzle/ColourLightBeams/BlueLightBeam_BP.BlueLightBeam_BP_C")
            (else
              (goto _label))))))
    (else
      (`ChildActorComponent.SetChildActorClass` _red "/Game/Blueprints/MirrorPuzzle/ColourLightBeams/RedLightBeam_BP.RedLightBeam_BP_C")
      (`ChildActorComponent.SetChildActorClass` _yellow "/Game/Blueprints/MirrorPuzzle/ColourLightBeams/YellowLightBeam_BP.YellowLightBeam_BP_C")
      (`ChildActorComponent.SetChildActorClass` _blue "/Game/Blueprints/MirrorPuzzle/ColourLightBeams/BlueLightBeam_BP.BlueLightBeam_BP_C"))))

(fn `UserConstructionScript`
  (`parent.UserConstructionScript`))