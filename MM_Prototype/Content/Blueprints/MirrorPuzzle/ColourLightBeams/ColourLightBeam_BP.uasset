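; Coloured light beam actor from the mirror puzzle, drawn as a glowing cylinder that reaches to whatever it hits.
; On BeginPlay, BeamColour selects the glow materials for the static mesh and cylinder.
; Each tick, a forward sphere trace finds a blocking hit and stretches the cylinder to it, with mixed colours drawn wider than primaries.
; The MirrorObject_BP cast on the hit actor triggers no logic.
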(event `self.ReceiveBeginPlay`
  (bind _beam_colour (`self.Beam Colour`))
  (`PrimitiveComponent.SetMaterial` (`self.StaticMesh`) 0 (select `/Game/Blueprints/MirrorPuzzle/ColourLightBeams/BeamColour_Enum` _beam_colour :`NewEnumerator0` "/Game/Materials/LightBeamMaterial/LightGlow_Mat_Red.LightGlow_Mat_Red" :`NewEnumerator1` "/Game/Materials/LightBeamMaterial/LightGlow_Mat_Yellow.LightGlow_Mat_Yellow" :`NewEnumerator2` "/Game/Materials/LightBeamMaterial/LightGlow_Mat_BLue.LightGlow_Mat_BLue" :`NewEnumerator3` "/Game/Materials/LightBeamMaterial/LightGlow_Mat_Orange.LightGlow_Mat_Orange" :`NewEnumerator4` "/Game/Materials/LightBeamMaterial/LightGlow_Mat_Purple.LightGlow_Mat_Purple" :`NewEnumerator5` "/Game/Materials/LightBeamMaterial/LightGlow_Mat_Green.LightGlow_Mat_Green" :!type "MaterialInterface Object Reference"))
  (`PrimitiveComponent.SetMaterial` (`self.Cylinder`) 0 (select `/Game/Blueprints/MirrorPuzzle/ColourLightBeams/BeamColour_Enum` _beam_colour :`NewEnumerator0` "/Game/Materials/LightBeamMaterial/LightGlow_Mat_RedOut.LightGlow_Mat_RedOut" :`NewEnumerator1` "/Game/Materials/LightBeamMaterial/LightGlow_Mat_Yellowout.LightGlow_Mat_Yellowout" :`NewEnumerator2` "/Game/Materials/LightBeamMaterial/LightGlow_Mat_BlueOut.LightGlow_Mat_BlueOut" :`NewEnumerator3` "/Game/Materials/LightBeamMaterial/LightGlow_Mat_OrangeOut.LightGlow_Mat_OrangeOut" :`NewEnumerator4` "/Game/Materials/LightBeamMaterial/LightGlow_Mat_PurpleOut.LightGlow_Mat_PurpleOut" :`NewEnumerator5` "/Game/Materials/LightBeamMaterial/LightGlow_Mat_GreenOut.LightGlow_Mat_GreenOut" :!type "MaterialInterface Object Reference")))

(event `self.ReceiveTick`
  (params (DeltaSeconds :type "Float (single-precision)"))
  (bind _returnvalue (`self.K2_GetActorLocation`))
  (bind _cylinder (`self.Cylinder`))
  (bind _cylinder_2 (`self.Cylinder`))
  (bind (_returnvalue_x _returnvalue_y _returnvalue_z) (`KismetMathLibrary.BreakVector` (`SceneComponent.K2_GetComponentScale` _cylinder_2)))
  (bind _returnvalue_2 (select `/Game/Blueprints/MirrorPuzzle/ColourLightBeams/BeamColour_Enum` (`self.Beam Colour`) :`NewEnumerator0` 0.33 :`NewEnumerator1` 0.33 :`NewEnumerator2` 0.33 :`NewEnumerator3` 0.6 :`NewEnumerator4` 0.6 :`NewEnumerator5` 0.6 :!type "Float (single-precision)"))
  (bind _outhit (`KismetSystemLibrary.SphereTraceSingle` :`Start` _returnvalue :`End` (+ _returnvalue (* (`SceneComponent.GetForwardVector` (`self.DefaultSceneRoot`)) 10000.0)) :`Radius` 15.0 :`TraceChannel` "TraceTypeQuery1" :`bTraceComplex` true :`TraceColor` (struct :`R` 1.0 :`G` 0.34375 :`B` 0.34375 :`A` 1.0) :`TraceHitColor` (struct :`R` 1.0 :`G` 0.739724 :`B` 0.071455 :`A` 1.0)))
  (bind (_bblockinghit _binitialoverlap _time _distance _location _impactpoint _normal _impactnormal _physmat _hitactor) (`GameplayStatics.BreakHitResult` _outhit))
  (if _bblockinghit
    (`SceneComponent.K2_SetWorldLocation` _cylinder (+ (/ _returnvalue 2.0) (/ _impactpoint 2.0)) false false)
    (`SceneComponent.SetWorldScale3D` _cylinder (`KismetMathLibrary.MakeVector` (.x (`SceneComponent.K2_GetComponentScale` (`self.Cylinder`))) (.y (`SceneComponent.K2_GetComponentScale` (`self.Cylinder`))) (* (`KismetMathLibrary.VSize` (- _returnvalue _impactpoint)) 0.01)))
    (cast `/Game/Blueprints/MirrorPuzzle/MirrorObject_BP` _hitactor
      (:`then`
        _)
      (:`CastFailed`
        _))
    (`SceneComponent.SetWorldScale3D` _cylinder_2 (`KismetMathLibrary.MakeVector` _returnvalue_2 _returnvalue_2 _returnvalue_z))))

(fn `UserConstructionScript`)