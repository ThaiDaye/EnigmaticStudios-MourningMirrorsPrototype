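; FallingPlatform is a platform that simulates falling away by disappearing after being touched, then respawning in place.
; Any overlap with its Box component starts a FallDelay, after which the StaticMesh loses collision and visibility without actually moving.
; After RespawnTime it restores both and resets a DoOnce gate, which blocks retriggering during the cycle.
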(event `self.Box.OnComponentBeginOverlap`
  (params (OverlappedComponent :type "PrimitiveComponent Object Reference") (OtherActor :type "Actor Object Reference") (OtherComp :type "PrimitiveComponent Object Reference") (OtherBodyIndex :type Integer) (bFromSweep :type Boolean) (SweepResult :type "HitResult Structure (by ref)"))
  (bind _staticmesh (`self.StaticMesh`))
  (bind _staticmesh_2 (`self.StaticMesh`))
  (`/Engine/EditorBlueprintResources/StandardMacros.DoOnce` false :!label _label
    (:`Completed`
      (`KismetSystemLibrary.Delay` (`self.FallDelay`))
      (`PrimitiveComponent.SetCollisionEnabled` _staticmesh_2 "NoCollision")
      (`SceneComponent.SetVisibility` _staticmesh_2 false true)
      (`KismetSystemLibrary.Delay` (`self.RespawnTime`))
      (`PrimitiveComponent.SetCollisionEnabled` _staticmesh "QueryAndPhysics")
      (`SceneComponent.SetVisibility` _staticmesh true true)
      (goto _label :!via `Reset`))))

(fn `UserConstructionScript`
  (`parent.UserConstructionScript`))