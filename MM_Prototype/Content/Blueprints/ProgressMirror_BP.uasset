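; Progress mirror that destroys itself once completed, or acts as a teleporter when flagged as a teleport mirror.
; When gem-activated, Tick completes it once every referenced gem is active.
; Interacting with a teleport mirror moves the character to another mirror with the same number.
; Otherwise, a delay-reopened Gate throttles interaction, which slots the character's shards up to the required count and completes the mirror when reached.
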(event `self.ReceiveTick`
  (params (DeltaSeconds :type "Float (single-precision)"))
  (`parent.ReceiveTick` DeltaSeconds)
  (if (`self.JemActivated`)
    (set `self.UnlockedRef` true)
    (for _array_element (`self.JemReferences`)
      (if (not (`/Game/FirstPersonBP/Blueprints/MirrorPuzzle/KeyJem_BP.Activated` _array_element))
        (set `self.UnlockedRef` false)))
    (if (`self.UnlockedRef`)
      (`KismetSystemLibrary.PrintString` "MIRROR COMPLETE" :!label _label)
      (`self.K2_DestroyActor`))))

(event `self.Interact`
  (bind _charref (`self.CharRef`))
  (bind _shardsobtained (`/Game/Blueprints/JasonHiscock_BP.ShardsObtained` _charref))
  (bind _returnvalue (`KismetMathLibrary.Clamp` (+ (`self.ShardsSlotted`) _shardsobtained) 0 (`self.Shards Required`)))
  (if (`self.TeleportMirror`)
    (bind _outactors (`GameplayStatics.GetAllActorsOfClass` "ProgressMirror_BP_C"))
    (for _array_element _outactors
      (if (and (`/Game/Blueprints/ProgressMirror_BP.TeleportMirror` _array_element) (== (`/Game/Blueprints/ProgressMirror_BP.TeleportNum` _array_element) (`self.TeleportNum`)) (not (== _array_element self)))
        (`self.K2_SetActorTransform` (`self.CharRef`) (`SceneComponent.K2_GetComponentToWorld` (`/Game/Blueprints/ProgressMirror_BP.Teleport Location` _array_element)) false true)))
    (else
      (`/Engine/EditorBlueprintResources/StandardMacros.Gate` false :!label _label_2
        (:`Exit`
          (`|ExecutionSequence`
            (:`then_0`
              (`|ExecutionSequence`
                (:`then_0`
                  (goto _label_2 :!via `Close`))
                (:`then_1`
                  (`KismetSystemLibrary.Delay` (`self.InteractDelay`))
                  (goto _label_2 :!via `Open`))))
            (:`then_1`
              (if (not (>= (`self.ShardsSlotted`) (`self.Shards Required`)))
                (set `self.ShardsSlotted` _returnvalue)
                (set `/Game/Blueprints/JasonHiscock_BP.ShardsObtained` (- _shardsobtained _returnvalue) _charref)
                (if (>= (`self.ShardsSlotted`) (`self.Shards Required`))
                  (goto _label)
                  (else
                    (`KismetSystemLibrary.PrintString` "MORE SHARDS REQUIRED")))))))))))

(fn `UserConstructionScript`
  (`parent.UserConstructionScript`))