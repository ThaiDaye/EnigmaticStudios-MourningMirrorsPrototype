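; LargeObject_BP is an interactable object whose appearance can change with the player's detective mode.
; When HiddenDetectiveMode is set, Tick shows Cube in detective mode and Sphere otherwise, reading JasonHiscock_BP from the player character each frame.
; Interact only runs a Gate-and-Delay cooldown, with no further action attached.
; BeginPlay caches the first JasonHiscock_BP in CharRef, which Tick does not use.
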(event `Interact`
  (`/Engine/EditorBlueprintResources/StandardMacros.Gate` false :!label _label
    (:`Exit`
      (`|ExecutionSequence`
        (:`then_0`
          (`|ExecutionSequence`
            (:`then_0`
              (goto _label :!via `Close`))
            (:`then_1`
              (`KismetSystemLibrary.Delay` (`self.InteractDelay`))
              (goto _label :!via `Open`))))
        (:`then_1`)))))

(event `self.ReceiveTick`
  (params (DeltaSeconds :type "Float (single-precision)"))
  (bind _detectivemode (`/Game/Blueprints/JasonHiscock_BP.DetectiveMode` (cast `/Game/Blueprints/JasonHiscock_BP` (`GameplayStatics.GetPlayerCharacter` 0) :!pure true)))
  (if (`self.HiddenDetectiveMode`)
    (`SceneComponent.SetHiddenInGame` (`self.Cube`) (not _detectivemode) true)
    (`SceneComponent.SetHiddenInGame` (`self.Sphere`) _detectivemode true)))

(event `self.ReceiveBeginPlay`
  (bind _outactors (`GameplayStatics.GetAllActorsOfClass` "/Game/Blueprints/JasonHiscock_BP.JasonHiscock_BP_C"))
  (set `self.CharRef` (`|GetArrayItem` _outactors)))

(fn `UserConstructionScript`)