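; BP_Movable is an interactable base or prop whose Cube can be revealed by the player's Detective Mode.
; BeginPlay caches the BP_Player reference, while Interact runs only a DoOnce gate that resets after InteractDelay, with no movement logic in this graph.
; When Invisible is set, Tick polls DetectiveMode on the player character and hides or shows the Cube and its children accordingly.
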(event `self.ReceiveBeginPlay`
  ;[1 1 1] Sets the Player Reference.
  (bind _outactors (`GameplayStatics.GetAllActorsOfClass` "/Game/MourningMirrorsVS/Core/Characters/BP_Player.BP_Player_C"))
  (set `self.PlayerRef` (`|GetArrayItem` _outactors)))

(event `Interact`
  ;[1 1 1] Interaction
  (`/Engine/EditorBlueprintResources/StandardMacros.DoOnce` false :!label _label ; Prevents further interaction \nuntil the delay has completed
    (:`Completed`
      (`KismetSystemLibrary.Delay` (`self.InteractDelay`))
      (`|ExecutionSequence`
        (:`then_0`
          (goto _label :!via `Reset`))))))

(event `self.ReceiveTick`
  (params (DeltaSeconds :type "Float (single-precision)"))
  ;[1 1 1] Checks whether the player is using Detective Mode if bInvisible is set to true.
  (if (`self.bInvisible`)
    (`SceneComponent.SetHiddenInGame` (`self.Cube`) (not (`/Game/MourningMirrorsVS/Core/Characters/BP_Player.DetectiveMode` (cast `/Game/MourningMirrorsVS/Core/Characters/BP_Player` (`GameplayStatics.GetPlayerCharacter` 0) :!pure true))) true)))

(fn `UserConstructionScript`)