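; BP_Swing is an interactable that shows a floating text prompt when targeted, with no swinging logic in this graph.
; BeginPlay caches the BP_Player tagged "Player" as the rotation target.
; Targeted sets IsBeingLookedAt, never cleared here, and shows the text briefly before hiding it.
; Tick rotates the text every frame, even while hidden, setting relative rotation from the player-to-text direction after zeroing world rotation.
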(event `self.ReceiveBeginPlay`
  ;[1 1 1] FetchPlayerReference
  (bind _outactors (`GameplayStatics.GetAllActorsOfClassWithTag` "/Game/MourningMirrorsVS/Core/Characters/BP_Player.BP_Player_C" "Player"))
  (for _array_element _outactors
    (set `self.TextRotationTarget` _array_element)))

(event `Targeted`
  (bind _textrender (`self.TextRender`))
  ;[1 1 1] Subroutine to run when player looks at the stalactight
  (set `self.IsBeingLookedAt` true)
  (`SceneComponent.SetVisibility` _textrender true false)
  (`KismetSystemLibrary.Delay` 0.1)
  (`SceneComponent.SetVisibility` _textrender false false))

(event `self.ReceiveTick`
  (params (DeltaSeconds :type "Float (single-precision)"))
  (bind _textrender (`self.TextRender`))
  ;[1 1 1] Controls Text Rotation (Could optimise by only rotating when text is displayed.)
  (if true
    (`SceneComponent.K2_SetWorldRotation` :`self` _textrender)
    (`SceneComponent.K2_SetRelativeRotation` _textrender (`KismetMathLibrary.Conv_VectorToRotator` (- (`SceneComponent.K2_GetComponentLocation` _textrender) (`self.K2_GetActorLocation` (`self.TextRotationTarget`)))) false false)))

(fn `UserConstructionScript`)